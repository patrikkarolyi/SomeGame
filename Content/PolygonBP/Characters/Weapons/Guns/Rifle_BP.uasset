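; Rifle weapon Blueprint that handles hitscan firing, reloading and reporting its aiming overlay state.
; Fire line-traces from the owning player's camera, damages actors implementing DamagableBPI, and plays impact effects and sounds while spending ammo.
; Reload refills the magazine from reserve ammo and updates the owner's ammo UI.
; The UI update in Fire is disconnected, so shots do not refresh the display.
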(fn ConstructionScript
  (|CallParentFunction))

(fn GetGunAimingOverlayState
  (return (Variables|Default|GetAimingOverlayState)))

(fn Fire
  (if (> (Variables|Default|GetCurrentAmmo) 0)
    ;[1 1 1] Get Camera
    (Variables|Default|GetPlayerCamera
      (:then
        _)
      (:else
        (Variables|Default|SetPlayerCamera (Actor|GetComponentbyClass (Variables|Default|GetOwnerPlayer) "/Script/Engine.CameraComponent"))))
    (bind _outhit (Collision|LineTraceByChannel (+ (Transformation|GetWorldLocation (Variables|Default|GetPlayerCamera)) (* (Math|Vector|GetForwardVector (Transformation|GetWorldRotation (Variables|Default|GetPlayerCamera))) 1.5e+02)) (+ (Transformation|GetWorldLocation (Variables|Default|GetPlayerCamera)) (* (Math|Vector|GetForwardVector (Transformation|GetWorldRotation (Variables|Default|GetPlayerCamera))) (Variables|Default|GetShotLength))) "TraceTypeQuery1" false 0 "None" true "(R=1.000000,G=0.000000,B=0.074020,A=1.000000)" "(R=0.000000,G=0.000000,B=0.000000,A=0.000000)" 0.05))
    ;[1 1 1] On Hit Damagable Target
    (if (Utilities|DoesObjectImplementInterface (.HitActor (Collision|BreakHitResult _outhit)) "/Game/PolygonBP/Characters/Weapons/DamagableBPI.DamagableBPI_C")
      (Class|DamagableBPI|DamageCharacter(Message) (.HitActor (Collision|BreakHitResult _outhit)) (Variables|Default|GetBulletDamage))
      (Effects|SpawnEmitteratLocation "/Game/PolygonHeist/ParticleFX/FX_Money.FX_Money" (.Location (Collision|BreakHitResult _outhit)))
      (else
        (Effects|SpawnEmitteratLocation "/Game/PolygonHeist/ParticleFX/FX_Gunshot.FX_Gunshot" (.Location (Collision|BreakHitResult _outhit)) "0, 0, 0" "0.500000,0.500000,0.500000")))
    (Audio|PlaySoundatLocation "/Game/PolygonBP/Characters/Weapons/Guns/rifle.rifle" (Transformation|GetWorldLocation (Variables|Default|GetArrow)) "0, 0, 0" 1.0 1.0 0.0 0 0 0)
    (bind _result (Math|Integer|DecrementInt (Variables|Default|GetCurrentAmmo)))
    (else
      (Audio|PlaySoundatLocation "/Game/PolygonBP/Characters/Weapons/Guns/noAmmo.noAmmo" (Transformation|GetWorldLocation (Variables|Default|GetArrow)) "0, 0, 0" 1.0 1.0 0.0 0 0 0))))

(fn Reload
  (bind _ownerplayer (Variables|Default|GetOwnerPlayer))
  (if (>= (+ (Variables|Default|GetAllAmmo) (Variables|Default|GetCurrentAmmo)) (Variables|Default|GetMaxAmmo))
    (bind _output_get (Variables|Default|SetAllAmmo (- (+ (Variables|Default|GetAllAmmo) (Variables|Default|GetCurrentAmmo)) (Variables|Default|GetMaxAmmo))))
    (bind _output_get_2 (Variables|Default|SetCurrentAmmo (Variables|Default|GetMaxAmmo)))
    (Default|UpdateAmmoUI _ownerplayer _output_get_2 _output_get)
    (else
      (bind _output_get_3 (Variables|Default|SetCurrentAmmo (+ (Variables|Default|GetAllAmmo) (Variables|Default|GetCurrentAmmo))))
      (bind _output_get_4 (Variables|Default|SetAllAmmo 0))
      (Default|UpdateAmmoUI _ownerplayer _output_get_3 _output_get_4))))