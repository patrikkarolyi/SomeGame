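; Gun projectile actor that flies at a set velocity and destroys itself on the first actor overlap.
; BeginPlay copies its Velocity variable into the ProjectileMovement component.
; On overlap it calls DestroyActor first, then calls ApplyDamage with a fixed amount if the other actor can be damaged, printing a debug YES or NO.
; The construction script tints the mesh with ProjectileColor through a dynamic material instance.
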(event EventBeginPlay
  (Variables|/Script/Engine.MovementComponent|SetVelocity (Variables|Default|GetProjectileMovement) (Variables|Default|GetVelocity)))

(event Collision|EventActorBeginOverlap
  (params (OtherActor :type Actor%20Object%20Reference))
  (Actor|DestroyActor)
  (if (Variables|/Script/Engine.Actor|GetbCanBeDamaged OtherActor)
    (Development|PrintString "YES")
    (Game|Damage|ApplyDamage 0 5e+01 0 0)
    (else
      (Development|PrintString "NO"))))

(fn ConstructionScript
  (bind _returnvalue (Rendering|Material|CreateDynamicMaterialInstance (Variables|Default|GetMesh) 0 0 "None" :!class /Script/Engine.PrimitiveComponent))
  (Rendering|Material|SetVectorParameterValue _returnvalue "Color" (Variables|Default|GetProjectileColor) :!class /Script/Engine.MaterialInstanceDynamic))